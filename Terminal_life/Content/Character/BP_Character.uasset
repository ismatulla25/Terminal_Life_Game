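; First-person player character that walks, interacts with objects, sits on a chair and operates an in-world computer.
; A timed sphere trace finds IBP_InteractedObject actors, animates the HUD use prompt and supplies the LMB target.
; Timelines lerp sitting and standing; screen mode locks movement and look, routing clicks through WidgetInteraction, while RMB backs out of each stage.
; Movement drives looping footstep sounds and walk/idle camera shake, while turning adds decaying camera tilt.
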(event Custom|Camera%20Shake
  (bind _returnvalue (Game|GetPlayerController 0))
  ;[1 0.5569 0.6275 0.502] Camera Shake
  (if (> (Math|Vector|VectorLength (Transformation|GetVelocity)) 2.0)
    (Game|Feedback|ClientStartCameraShake _returnvalue "/Game/Character/CameraShake/CameraShake_Walk.CameraShake_Walk_C" 1.0 "CameraLocal" "0, 0, 0")
    (else
      (Game|Feedback|ClientStartCameraShake _returnvalue "/Game/Character/CameraShake/CameraShake_Idle.CameraShake_Idle_C" 1.0 "CameraLocal" "0, 0, 0"))))

(event Custom|FootStapsSound
  ;[0.5501 1 0.9602 0.5] FootStepsSound
  (Audio|Components|Audio|Play (Variables|Default|GetFootSteps) 0.0))

(event Custom|LineTrace
  (bind _characterinterface (Variables|Default|GetCharacterInterface))
  ;[1 0.5569 0.6275 0.502] Use UI Animation
  (CallFunction|LineTrace)
  (if (Variables|Default|GetObjectHaveUseInterface)
    (Utilities|FlowControl|DoOnce false :!label _label
      (:Completed
        (UserInterface|Animation|PlayAnimation _characterinterface (Variables|/Game/Character/WBP_CharacterInterface.WBP_CharacterInterface_C|GetUSE_TextAnimation1 _characterinterface) 0.0 1 "Forward" 1.0 false)
        (goto _label_2 Reset)))
    (else
      (Utilities|FlowControl|DoOnce false :!label _label_2
        (:Completed
          (UserInterface|Animation|PlayAnimation _characterinterface (Variables|/Game/Character/WBP_CharacterInterface.WBP_CharacterInterface_C|GetUSE_TextAnimation0 _characterinterface) 0.0 1 "Forward" 1.0 false)
          (goto _label Reset))))))

(event EventAroowLocationRotation
  (params (AroowTransform :type Transform) (StulArrowTransform :type Transform) (Computer :type Actor%20Object%20Reference))
  ;[0.15 0.15 0.15 0.5] StartInfo
  (Utilities|FlowControl|Sequence
    (:then_0
      (Utilities|FlowControl|DoOnce false
        (:Completed
          (Variables|Default|SetArrow%20Location/%20Rotation AroowTransform)
          (Variables|Default|SetComputer Computer))))))

(event EventTick
  (params (DeltaSeconds :type Float%20%28single-precision%29))
  (Utilities|FlowControl|Sequence
    (:then_0
      ;[1 0.5569 0.6275 0.502] Camera Animation
      (if (not (Variables|Default|GetAtTheScreen))
        (CallFunction|CameraShake)
        (Variables|Default|SetTilt (Math|Float|SelectFloat (Math|Float|Clamp(Float) (- (Variables|Default|GetTilt) (* (Variables|Default|GetTilt) (Variables|Default|GetTiltRecoverSpeed) DeltaSeconds)) (* (Variables|Default|GetMaxTilt) -1.0) 0.0) (Math|Float|Clamp(Float) (- (Variables|Default|GetTilt) (* (Variables|Default|GetTilt) (Variables|Default|GetTiltRecoverSpeed) DeltaSeconds)) 0.0 (Variables|Default|GetMaxTilt)) (< (- (Variables|Default|GetTilt) (* (Variables|Default|GetTilt) (Variables|Default|GetTiltRecoverSpeed) DeltaSeconds)) 0.0)))
        (if (Variables|Default|GetSpringArmAnim)
          (Transformation|SetWorldRotation (Variables|Default|GetSpringArm) (Pawn|GetControlRotation (Pawn|GetController) :!class /Script/Engine.Controller) false false)
          (Transformation|AddRelativeRotation (Variables|Default|GetSpringArm) (Math|Rotator|MakeRotator (Variables|Default|GetTilt) 0.0 0.0) false false))))))

(event EventUSE
  (params (TraceComponent :type Actor%20Component%20Object%20Reference))
  (bind _stultransform (Variables|Default|GetStulTransform))
  ;[0 0 0 0.5] Key E (SitOnTheComputer) / Key ESC (Exit/Undo)
  (if (not (Variables|Default|GetSIt?))
    (Collision|SetCollisionEnabled (Variables|Collision|GetCapsuleComponent) "ProbeOnly")
    (Variables|/Script/Engine.MovementComponent|SetVelocity (Variables|Character|GetCharacterMovement) "0, 0, 0")
    (Variables|Default|SetSpringArmAnim false)
    (Utilities|FlowControl|Delay 0.3)
    (Variables|/Script/Engine.SpringArmComponent|SetbUsePawnControlRotation (Variables|Default|GetSpringArm) true)
    (bind (_direction _location _rotation) (Timeline|ActorLerp-L/R PlayFromStart)
      (:Update
        (Pawn|SetControlRotation (Game|GetPlayerController 0) (Math|Interpolation|RInterpTo (Transformation|GetWorldRotation (Variables|Default|GetSpringArm)) (Math|Rotator|MakeRotator (.roll (.rotation _stultransform)) (.pitch (.rotation _stultransform)) (+ (.yaw (.rotation _stultransform)) -9e+01)) _rotation 3.0))
        (Transformation|SetActorLocation (Math|Vector|Lerp(Vector) (Transformation|GetActorLocation) (.location (Variables|Default|GetStulTransform)) _location) false false)
        (Variables|Default|SetLTLeth 2e+02))
      (:Finished
        (Development|PrintString "ACE")
        (bind _output_get (Variables|Default|SetSIt? true))
        (Class|IBPBoolVarSIT|SitInfoforComputer(Message) (Variables|Default|GetComputer) _output_get)
        (Variables|Default|SetSpringArmAnim true)
        (Variables|/Script/Engine.SpringArmComponent|SetbUsePawnControlRotation (Variables|Default|GetSpringArm) false)))))

(event EventStullRotation
  (params (StulArrowTransform :type Transform) (BP_Stul :type Actor%20Object%20Reference) (OnTheStul :type Boolean))
  ;[0.15 0.15 0.15 0.5] StartInfo
  (Utilities|FlowControl|Sequence
    (:then_0
      (Utilities|FlowControl|DoOnce false
        (:Completed
          (Variables|Default|SetBP_Stul BP_Stul))))
    (:then_1
      (Variables|Default|SetStulTransform StulArrowTransform))))

(event EventBeginPlay
  (Utilities|FlowControl|Sequence
    (:then_0
      ;[0.15 0.15 0.15 0.5] StartNode
      (bind _returnvalue (UserInterface|CreateWidget "/Game/Blueprints/Computer/WidgetInterface/WBP_ComputerInterface.WBP_ComputerInterface_C"))
      (Variables|Default|SetComputerInterface _returnvalue)
      (bind _returnvalue_2 (UserInterface|CreateWidget "/Game/Character/WBP_CharacterInterface.WBP_CharacterInterface_C"))
      (bind _output_get (Variables|Default|SetCharacterInterface _returnvalue_2))
      (UserInterface|Viewport|AddtoViewport _output_get 0))
    (:then_1
      ;[1 0.5569 0.6275 0.502] Use UI Animation
      (Utilities|Time|SetTimerbyEvent (delegate Custom|LineTrace) 0.1 true))))

(event Input|ActionEvents|InputActionInteractedLMB
  (params (Key :type Key%20Structure :default "None"))
  (bind _returnvalue (Game|GetPlayerController 0))
  (bind _cursorposition (Variables|Default|GetCursorPosition))
  (bind _arrow_location__rotation (Variables|Default|GetArrow%20Location/%20Rotation))
  (bind (_x _y _z) (Math|Vector|BreakVector (.location _arrow_location__rotation)))
  ;[0.1412 0.07843 0.08627 0.502] InteractOnTheComputerMonitor LMB
  (:Pressed
    (if (Variables|Default|GetSIt?)
      (if (not (Variables|Default|GetAtTheScreen))
        (if (== "/Game/Blueprints/Computer/BP_Computer.BP_Computer_C" (Utilities|GetClass (Variables|Default|GetTraceObject)))
          (Variables|Default|SetAtTheScreen true)
          (Utilities|FlowControl|Sequence
            (:then_0
              (Transformation|SetActorLocation (Math|Vector|MakeVector _x (- _y 8e+01) _z) false false)
              (Class|PlayerController|SetMouseLocation (Game|GetPlayerController 0) (Math|Float|Truncate (.x _cursorposition)) (Math|Float|Truncate (.y _cursorposition)))
              (Pawn|SetControlRotation (Game|GetPlayerController 0) (.rotation (Variables|Default|GetArrow%20Location/%20Rotation)))
              (Variables|/Script/Engine.PlayerController|SetbShowMouseCursor (Game|GetPlayerController 0) false)
              (Variables|/Script/Engine.PostProcessComponent|SetbEnabled (Variables|Default|GetPostProcess2) true)
              (Widget|RemovefromParent (Variables|Default|GetCharacterInterface))
              (Input|SetIgnoreLookInput _returnvalue true)
              (Input|SetIgnoreMoveInput _returnvalue true))
            (:then_1
              (Utilities|FlowControl|Delay 0.2)
              (Transformation|SetRelativeRotation (Variables|Default|GetSpringArm) (Math|Rotator|MakeRotator 0.0 0.0 0.0) false false))))))))

(event Input|ActionEvents|InputActionInteractedLMB
  (params (Key :type Key%20Structure :default "None"))
  ;[0 0 0 0.5] UseObject LMB
  (:Pressed
    (Class|IBPUSE|USE(Message) (Variables|Default|GetTraceObject) (Variables|Default|GetTraceComponent))))

(event Input|ActionEvents|InputActionInteractedLMB
  (params (Key :type Key%20Structure :default "None"))
  (bind _widgetinteraction (Variables|Default|GetWidgetInteraction))
  ;[0.1412 0.07843 0.08627 0.502] InteractOnTheComputerMonitor LMB
  (:Pressed
    (if (Variables|Default|GetAtTheScreen)
      (Class|WidgetInteractionComponent|PressPointerKey _widgetinteraction Key)))
  (:Released
    (if (Variables|Default|GetAtTheScreen)
      (Class|WidgetInteractionComponent|ReleasePointerKey _widgetinteraction Key))))

(event Input|ActionEvents|InputActionExitFromComputerRMB
  (params (Key :type Key%20Structure :default "None"))
  (bind _returnvalue (Game|GetPlayerController 0))
  (bind _returnvalue_2 (Game|GetPlayerController 0))
  (bind _stultransform (Variables|Default|GetStulTransform))
  (bind (_locationx _locationy) (Game|Player|GetMousePosition _returnvalue_2))
  (bind _returnvalue_3 (Math|Vector|GetForwardVector (.rotation _stultransform)))
  (bind _returnvalue_4 (* _returnvalue_3 65))
  (bind _returnvalue_5 (+ (.location _stultransform) _returnvalue_4))
  ;[0 0 0 0.5] Key E (SitOnTheComputer) / Key ESC (Exit/Undo)
  (:Pressed
    (if (Variables|Default|GetAtTheScreen)
      (if (Variables|Default|GetSIt?)
        (Input|SetIgnoreLookInput _returnvalue false)
        (Input|SetIgnoreMoveInput _returnvalue false)
        (UserInterface|Viewport|AddtoViewport (Variables|Default|GetCharacterInterface) 0)
        (Variables|Default|SetCursorPosition (Math|Vector|MakeVector _locationx _locationy 0.0))
        (Variables|/Script/Engine.PostProcessComponent|SetbEnabled (Variables|Default|GetPostProcess2) false)
        (Variables|/Script/Engine.PlayerController|SetbShowMouseCursor (Game|GetPlayerController 0) false)
        (Variables|Default|SetAtTheScreen false)
        (Transformation|SetActorLocation (.location (Variables|Default|GetStulTransform)) false false)
        (Pawn|SetControlRotation (Game|GetPlayerController 0) (.rotation (Variables|Default|GetArrow%20Location/%20Rotation))))
      (elif (Variables|Default|GetSIt?)
        (Class|IBPUSE|USE(Message) (Variables|Default|GetBP_Stul))
        (Variables|Default|SetSIt? false)
        (bind _standuplocation (Timeline|StendUp PlayFromStart)
          (:Update
            (Transformation|SetActorLocation (Math|Vector|Lerp(Vector) (Transformation|GetActorLocation) (Math|Vector|MakeVector (.x _returnvalue_5) (.y _returnvalue_5) 1e+02) _standuplocation) false false))
          (:Finished
            (Collision|SetCollisionEnabled (Variables|Collision|GetCapsuleComponent) "QueryAndPhysics")
            (Class|IBPBoolVarSIT|SitInfoforComputer(Message) (Variables|Default|GetComputer) (Variables|Default|GetSIt?))
            (Variables|Default|SetLTLeth 125.0)))))))

(event Input|AxisEvents|InputAxisMoveForward
  (params (AxisValue :type Float%20%28single-precision%29))
  ;[0 0 0 0.5] Move
  (Pawn|Input|AddMovementInput (Transformation|GetActorForwardVector) AxisValue false)
  ;[0.5501 1 0.9602 0.5] FootStepsSound
  (if (> (Math|Vector|VectorLength (Transformation|GetVelocity)) 1.0)
    (Variables|Default|SetFS_Loop true)
    (Utilities|FlowControl|DoOnce false :!label _label
      (:Completed
        _))
    (else
      (Utilities|FlowControl|Sequence
        (:then_0
          (goto _label Reset))
        (:then_1
          (Variables|Default|SetFS_Loop false)))))
  (Utilities|Time|SetTimerbyEvent (delegate Custom|FootStapsSound) 0.5 (Variables|Default|GetFS_Loop) true))

(event Input|AxisEvents|InputAxisMoveRight
  (params (AxisValue :type Float%20%28single-precision%29))
  ;[0 0 0 0.5] Move
  (Pawn|Input|AddMovementInput (Transformation|GetActorRightVector) AxisValue false)
  ;[0.5501 1 0.9602 0.5] FootStepsSound
  (if (> (Math|Vector|VectorLength (Transformation|GetVelocity)) 1.0)
    (Variables|Default|SetFS_Loop true)
    (Utilities|FlowControl|DoOnce false :!label _label
      (:Completed
        _))
    (else
      (Utilities|FlowControl|Sequence
        (:then_0
          (goto _label Reset))
        (:then_1
          (Variables|Default|SetFS_Loop false)))))
  (Utilities|Time|SetTimerbyEvent (delegate Custom|FootStapsSound) 0.5 (Variables|Default|GetFS_Loop) true))

(event Input|AxisEvents|InputAxisTurn
  (params (AxisValue :type Float%20%28single-precision%29))
  ;[0 0 0 0.5] Look (TiltRotation)
  (Pawn|Input|AddControllerYawInput AxisValue)
  (Variables|Default|SetTilt (+ AxisValue (Variables|Default|GetTilt))))

(event Input|AxisEvents|InputAxisLookUp
  (params (AxisValue :type Float%20%28single-precision%29))
  ;[0 0 0 0.5] Look (TiltRotation)
  (Pawn|Input|AddControllerPitchInput AxisValue))

(fn ConstructionScript)

(fn LineTrace
  (bind _camera (Variables|Default|GetCamera))
  (bind _returnvalue (Transformation|GetWorldLocation _camera))
  (bind _outhit (Collision|SphereTraceByChannel _returnvalue (+ _returnvalue (* (Math|Vector|GetForwardVector (Transformation|GetWorldRotation _camera)) (Variables|Default|GetLTLeth))) 8.0 "TraceTypeQuery1" false 0 "None" true "(R=1.000000,G=0.000000,B=0.000000,A=1.000000)" "(R=0.000000,G=1.000000,B=0.000000,A=1.000000)" 0.5))
  (if (Utilities|DoesObjectImplementInterface (.HitActor (Collision|BreakHitResult _outhit)) "/Game/Blueprints/IBP_InteractedObject.IBP_InteractedObject_C")
    (bind _canuse_o (Class|IBPInteractedObject|CanInteractedInterfaceAnim(Message) (.HitActor (Collision|BreakHitResult _outhit))))
    (bind _output_get (Variables|Default|SetObjectHaveUseInterface _canuse_o))
    (if _output_get
      (Variables|Default|SetTraceComponent (.HitComponent (Collision|BreakHitResult _outhit)))
      (Variables|Default|SetTraceObject (.HitActor (Collision|BreakHitResult _outhit)))
      (else
        (Variables|Default|SetTraceComponent 0)
        (Variables|Default|SetTraceObject 0)))
    (else
      (Variables|Default|SetObjectHaveUseInterface false)
      (Variables|Default|SetTraceObject 0)
      (Variables|Default|SetTraceComponent 0))))

(fn CanInteractedInterfaceAnim
  (return false))