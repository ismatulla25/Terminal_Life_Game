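; Interactable digital clock that shows hours and minutes on four digit meshes and can sound audio that the player switches off.
; A looping one-minute timer advances the time, wrapping hours from 11 to 0, and SetDigit picks each digit from a texture atlas through material UV offsets.
; ClockTurnON starts the audio after a random delay, and USE stops it with a button click sound.
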(event Custom|SetTime
  (CallFunction|SetDigit (/ (Variables|Default|GetCurrentHour) 10) (Variables|Default|GetTableNumber1))
  (CallFunction|SetDigit (Math|Integer|%(Integer) (Variables|Default|GetCurrentHour) 10) (Variables|Default|GetTableNumber2))
  (CallFunction|SetDigit (/ (Variables|Default|GetCurrentMinute) 10) (Variables|Default|GetTableNumber3))
  (CallFunction|SetDigit (Math|Integer|%(Integer) (Variables|Default|GetCurrentMinute) 10) (Variables|Default|GetTableNumber4))
  (bind _output_get (Variables|Default|SetCurrentMinute (+ (Variables|Default|GetCurrentMinute) 1)))
  (if (>= _output_get 60)
    (Variables|Default|SetCurrentMinute 0)
    (bind _output_get_2 (Variables|Default|SetCurrentHour (+ (Variables|Default|GetCurrentHour) 1)))
    (if (>= _output_get_2 12)
      (Variables|Default|SetCurrentHour 0))))

(event EventClockTurnON
  (Utilities|FlowControl|Delay (Math|Random|RandomFloatinRange 2.0 1e+01))
  (Audio|Components|Audio|Play (Variables|Default|GetAudio) 0.0))

(event EventBeginPlay
  (bind _plane (Variables|Default|GetPlane))
  (Rendering|Material|SetScalarParameterValueonMaterials _plane "Offset U" 60.5)
  (Rendering|Material|SetScalarParameterValueonMaterials _plane "Offset V" 2e+01)
  (Rendering|Material|SetScalarParameterValueonMaterials _plane "UVScale" 0.02)
  (Utilities|FlowControl|Sequence
    (:then_0
      (Utilities|Time|SetTimerbyEvent (delegate Custom|SetTime) 6e+01 true))
    (:then_1
      (CallFunction|SetDigit (/ (Variables|Default|GetCurrentHour) 10) (Variables|Default|GetTableNumber1))
      (CallFunction|SetDigit (Math|Integer|%(Integer) (Variables|Default|GetCurrentHour) 10) (Variables|Default|GetTableNumber2))
      (CallFunction|SetDigit (/ (Variables|Default|GetCurrentMinute) 10) (Variables|Default|GetTableNumber3))
      (CallFunction|SetDigit (Math|Integer|%(Integer) (Variables|Default|GetCurrentMinute) 10) (Variables|Default|GetTableNumber4))
      (bind _output_get (Variables|Default|SetCurrentMinute (+ (Variables|Default|GetCurrentMinute) 1)))
      (if (>= _output_get 60)
        (Variables|Default|SetCurrentMinute 0)
        (bind _output_get_2 (Variables|Default|SetCurrentHour (+ (Variables|Default|GetCurrentHour) 1)))
        (if (>= _output_get_2 12)
          (Variables|Default|SetCurrentHour 0))))))

(event EventUSE
  (params (TraceComponent :type Actor%20Component%20Object%20Reference))
  (Audio|Components|Audio|Stop (Variables|Default|GetAudio))
  (Audio|Components|Audio|Play (Variables|Default|GetButtonClick) 0.0))

(fn ConstructionScript)

(fn SetDigit
  (params (Digit :type Integer) (TargetMesh :type Static%20Mesh%20Component%20Object%20Reference))
  (switch int Digit
    (:0
      ;[0.1034 0.9531 0.3359 0.5] Number 0
      (Rendering|Material|SetScalarParameterValueonMaterials TargetMesh "Offset U" 0.8)
      (Rendering|Material|SetScalarParameterValueonMaterials TargetMesh "Offset V" 0.5)
      (return))
    (:1
      ;[0.1034 0.9531 0.3359 0.5] Number 1
      (Rendering|Material|SetScalarParameterValueonMaterials TargetMesh "Offset U" 0.0)
      (Rendering|Material|SetScalarParameterValueonMaterials TargetMesh "Offset V" 0.0)
      (return))
    (:2
      ;[0.1034 0.9531 0.3359 0.5] Number 2
      (Rendering|Material|SetScalarParameterValueonMaterials TargetMesh "Offset U" 0.2)
      (Rendering|Material|SetScalarParameterValueonMaterials TargetMesh "Offset V" 0.0)
      (return))
    (:3
      ;[0.1034 0.9531 0.3359 0.5] Number 3
      (Rendering|Material|SetScalarParameterValueonMaterials TargetMesh "Offset U" 0.4)
      (Rendering|Material|SetScalarParameterValueonMaterials TargetMesh "Offset V" 0.0)
      (return))
    (:4
      ;[0.1034 0.9531 0.3359 0.5] Number 4
      (Rendering|Material|SetScalarParameterValueonMaterials TargetMesh "Offset U" 0.6)
      (Rendering|Material|SetScalarParameterValueonMaterials TargetMesh "Offset V" 0.0)
      (return))
    (:5
      ;[0.1034 0.9531 0.3359 0.5] Number 5
      (Rendering|Material|SetScalarParameterValueonMaterials TargetMesh "Offset U" 0.8)
      (Rendering|Material|SetScalarParameterValueonMaterials TargetMesh "Offset V" 0.0))
    (:6
      ;[0.1034 0.9531 0.3359 0.5] Number 6
      (Rendering|Material|SetScalarParameterValueonMaterials TargetMesh "Offset U" 0.0)
      (Rendering|Material|SetScalarParameterValueonMaterials TargetMesh "Offset V" 0.5))
    (:7
      ;[0.1034 0.9531 0.3359 0.5] Number 7
      (Rendering|Material|SetScalarParameterValueonMaterials TargetMesh "Offset U" 0.2)
      (Rendering|Material|SetScalarParameterValueonMaterials TargetMesh "Offset V" 0.5)
      (return))
    (:8
      ;[0.1034 0.9531 0.3359 0.5] Number 8
      (Rendering|Material|SetScalarParameterValueonMaterials TargetMesh "Offset U" 0.4)
      (Rendering|Material|SetScalarParameterValueonMaterials TargetMesh "Offset V" 0.5)
      (return))
    (:9
      ;[0.1034 0.9531 0.3359 0.5] Number 9
      (Rendering|Material|SetScalarParameterValueonMaterials TargetMesh "Offset U" 0.6)
      (Rendering|Material|SetScalarParameterValueonMaterials TargetMesh "Offset V" 0.5)
      (return))))

(fn CanInteractedInterfaceAnim
  (return (Variables|Default|GetCanInteracted)))