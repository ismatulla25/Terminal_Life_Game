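; BP_Chandelier is a chandelier with a fan whose rotation speed is driven through its animation Blueprint, ABP_Chandelier.
; On BeginPlay it caches the anim instance and starts a looping timer that polls the FanONOFF flag.
; While the flag is on, the timer copies FanSpeed into the anim instance's RotationSpeed.
; While off, it zeroes only FanSpeed, leaving RotationSpeed at its last value.
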(event Custom|On
  (if (Variables|Default|GetFanON/OFF)
    (Variables|/Game/Blueprints/Chandelier/ABP_Chandelier.ABP_Chandelier_C|SetRotationSpeed (Variables|Default|GetAs%20ABP%20Chandelier) (Variables|Default|GetFanSpeed))
    (else
      (Variables|Default|SetFanSpeed 0.0))))

(event EventBeginPlay
  (bind _asabp_chandelier (Utilities|Casting|CastToABP_Chandelier (Components|SkeletalMesh|GetAnimInstance (Variables|Default|GetChandelier))))
  (Variables|Default|SetAs%20ABP%20Chandelier _asabp_chandelier)
  (Utilities|Time|SetTimerbyEvent (delegate Custom|On) 0.1 true))

(fn ConstructionScript)