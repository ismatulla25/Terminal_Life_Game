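; Journal actor that animates a book falling, then shows it open.
; BeginPlay caches a start transform from MainBook's relative transform, offset along Y.
; The JournalFall event waits briefly, then the Fall timeline lerps MainBook from that transform to TransformForAnim.
; When the timeline finishes, it plays FallSound and swaps visibility from MainBook to MainOpenBook.
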(event EventJournalFall
  (Utilities|FlowControl|Delay 1.0)
  (bind _fall (Timeline|Fall PlayFromStart)
    (:Update
      (Transformation|SetRelativeTransform (Variables|Default|GetMainBook) (Math|Transform|Lerp(Transform) (Variables|Default|GetFirstTransform) (Variables|Default|GetTransformForAnim) _fall) false false))
    (:Finished
      (Audio|Components|Audio|Play (Variables|Default|GetFallSound) 0.0)
      (Rendering|SetVisibility (Variables|Default|GetMainBook) false false)
      (Rendering|SetVisibility (Variables|Default|GetMainOpenBook) true false))))

(event EventBeginPlay
  (bind _mainbook (Variables|Default|GetMainBook))
  (bind _returnvalue (Transformation|GetRelativeTransform _mainbook))
  (Variables|Default|SetFirstTransform (Math|Transform|MakeTransform (Math|Vector|MakeVector (.x (.location _returnvalue)) (+ (.y (.location _returnvalue)) 25.0) (.z (.location _returnvalue))) (.rotation _returnvalue) (.scale _returnvalue))))

(fn ConstructionScript)