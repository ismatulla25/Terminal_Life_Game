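; BP_Wardrobe is an interactable wardrobe whose doors open and close when used.
; The USE event alternates through a FlipFlop between non-looping open and close animations on the Wardrobe component.
; Each animation plays only if none is running, but the FlipFlop still toggles on ignored uses.
; Can Interacted Interface Anim exposes the CanInteracted flag, which USE itself does not check.
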(event EventUSE
  (params (TraceComponent :type Actor%20Component%20Object%20Reference))
  (bind _wardrobe (Variables|Default|GetWardrobe))
  (bind _returnvalue (Audio|Components|Audio|IsPlaying _wardrobe))
  (Utilities|FlowControl|FlipFlop
    (:A
      (if (not _returnvalue)
        (Components|Animation|PlayAnimation (Variables|Default|GetWardrobe) "/Game/Blueprints/Wardrobe/Animations/Wardrobe_Anim_Armature_OpenDoors_Anim.Wardrobe_Anim_Armature_OpenDoors_Anim" false)))
    (:B
      (if (not _returnvalue)
        (Components|Animation|PlayAnimation (Variables|Default|GetWardrobe) "/Game/Blueprints/Wardrobe/Animations/Wardrobe_Anim_Armature_CloseDoors_Anim.Wardrobe_Anim_Armature_CloseDoors_Anim" false)))))

(fn ConstructionScript)

(fn CanInteractedInterfaceAnim
  (return (Variables|Default|GetCanInteracted?)))