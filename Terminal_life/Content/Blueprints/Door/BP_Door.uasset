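; BP_Door is an animated door Blueprint that opens after a random delay and can then be used to close it.
; OpenDoor waits a few seconds, sets CanUse, plays the open sound and the skeletal open animation.
; USE clears CanUse and plays the close animation, while an interface function exposes CanUse as the interaction check.
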(event EventOpenDoor
  (Utilities|FlowControl|Delay (Math|Random|RandomFloatinRange 2.0 1e+01))
  (Variables|Default|SetCanUse? true)
  (Audio|Components|Audio|Play (Variables|Default|GetDoorOpenAudio) 0.0)
  (Components|Animation|PlayAnimation (Variables|Default|GetMainDoor) "/Game/Blueprints/Door/Model/Animation/MainDoor_Anim_DoorArmature_OpenMainDoorAnim.MainDoor_Anim_DoorArmature_OpenMainDoorAnim" false))

(event EventUSE
  (params (TraceComponent :type Actor%20Component%20Object%20Reference))
  (Variables|Default|SetCanUse? false)
  (Components|Animation|PlayAnimation (Variables|Default|GetMainDoor) "/Game/Blueprints/Door/Model/Animation/MainDoor_Anim_DoorArmature_CloseMainDoorAnim.MainDoor_Anim_DoorArmature_CloseMainDoorAnim" false))

(fn ConstructionScript)

(fn CanInteractedInterfaceAnim
  (return (Variables|Default|GetCanUse?)))