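; BP_Computer is an interactable computer that can only be used while its OnTheStul seated flag is set.
; On BeginPlay it starts a working-PC sound, sends its Arrow transform and self-reference to the player character, and passes itself to the linked chair (BPStul).
; SitInfoforComputer updates the seated flag, which the CanInteractedInterfaceAnim check returns.
; VoiceMail plays any supplied sound through the Voice audio component.
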(event EventBeginPlay
  (Class|IBPAroowLR|AroowLocationRotation(Message) :self (Game|GetPlayerCharacter 0) :AroowTransform (Transformation|GetWorldTransform (Variables|Default|GetArrow)) :Computer self)
  (Class|IBPAroowLR|AroowLocationRotation(Message) :self (Variables|Default|GetBP%20Stul) :Computer self)
  (Audio|Components|Audio|Play (Variables|Default|GetPCWorkSound) 0.0))

(event EventSitInfoforComputer
  (params (Sit :type Boolean))
  (Variables|Default|SetOnTheStul? Sit))

(event EventVoiceMail
  (params (Voice :type Sound%20Base%20Object%20Reference))
  (Audio|Components|Audio|SetSound (Variables|Default|GetVoice) Voice)
  (Audio|Components|Audio|Play (Variables|Default|GetVoice) 0.0))

(fn ConstructionScript)

(fn CanInteractedInterfaceAnim
  (if (Variables|Default|GetOnTheStul?)
    (return true)
    (else
      (return false))))