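; Interactable swivel armchair that the player toggles between sitting in and leaving with USE.
; It messages the player character with the seat bone transform on sitting and the arrow's transform on leaving.
; On sitting, a timeline turns the chair's AB_ChairRotation anim instance toward the player, then a looping timer matches player rotation with a 90-degree yaw offset until exit.
; Its interact-animation interface check returns false while seated.
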(event Custom|StulRotation
  (bind _returnvalue (Game|GetPlayerCharacter 0))
  (bind _returnvalue_2 (Transformation|GetActorRotation _returnvalue))
  (bind (_roll _pitch _yaw) (Math|Rotator|BreakRotator _returnvalue_2))
  (Variables|/Game/Blueprints/Computer/Model/Armchair/AB_ChairRotation.AB_ChairRotation_C|SetChair%20Rotation (Variables|Default|GetAs%20AB%20Chair%20Rotation) (Math|Rotator|MakeRotator _roll _pitch (+ _yaw 9e+01))))

(event EventBeginPlay
  (Class|IBPStulRotation|StullRotation(Message) (Game|GetPlayerCharacter 0) (Transformation|GetBoneTransform (Variables|Default|GetArmchair) "ArmchairUP" "RTS_World") self (Variables|Default|GetIs%20sit?))
  (bind _asab_chair_rotation (Utilities|Casting|CastToAB_ChairRotation (Components|SkeletalMesh|GetAnimInstance (Variables|Default|GetArmchair))))
  (Variables|Default|SetAs%20AB%20Chair%20Rotation _asab_chair_rotation))

(event EventUSE
  (params (TraceComponent :type Actor%20Component%20Object%20Reference))
  (bind _returnvalue (Game|GetPlayerCharacter 0))
  (bind _armchair (Variables|Default|GetArmchair))
  (bind _armchair_2 (Variables|Default|GetArmchair))
  (bind _returnvalue_2 (Transformation|GetWorldLocation _armchair_2))
  (bind _returnvalue_3 (Transformation|GetActorLocation _returnvalue))
  (bind _returnvalue_4 (Transformation|GetBoneTransform _armchair "ArmchairUP" "RTS_World"))
  (bind _returnvalue_5 (Math|Rotator|FindLookatRotation _returnvalue_2 _returnvalue_3))
  (bind _yaw (Math|Rotator|BreakRotator _returnvalue_5))
  (bind _returnvalue_6 (+ _yaw 9e+01))
  (bind _returnvalue_7 (Math|Rotator|MakeRotator 0.0 0.0 _returnvalue_6))
  (Utilities|FlowControl|FlipFlop
    (:A
      (Variables|Default|SetIs%20sit? true)
      (Class|IBPStulRotation|StullRotation(Message) (Game|GetPlayerCharacter 0) (Math|Transform|MakeTransform (.location _returnvalue_4) _returnvalue_7 (.scale _returnvalue_4)) 0 (Variables|Default|GetIs%20sit?))
      (Class|IBPUSE|USE(Message) (Game|GetPlayerCharacter 0))
      (Utilities|FlowControl|Sequence
        (:then_0
          (Utilities|FlowControl|Delay 0.7)
          (bind _returnvalue_8 (Utilities|Time|SetTimerbyEvent (delegate Custom|StulRotation) 0.01 true)))
        (:then_1
          (bind _stulrotation (Timeline|StulRotator PlayFromStart)
            (:Update
              (Variables|/Game/Blueprints/Computer/Model/Armchair/AB_ChairRotation.AB_ChairRotation_C|SetChair%20Rotation (Variables|Default|GetAs%20AB%20Chair%20Rotation) (Math|Interpolation|RInterpTo (.rotation (Transformation|GetBoneTransform (Variables|Default|GetArmchair) "ArmchairUP" "RTS_World")) _returnvalue_7 _stulrotation 1.0)))))))
    (:B
      (Variables|Default|SetIs%20sit? false)
      (Class|IBPStulRotation|StullRotation(Message) (Game|GetPlayerCharacter 0) (Transformation|GetWorldTransform (Variables|Default|GetArrow%20Stul)) 0 (Variables|Default|GetIs%20sit?))
      (Utilities|Time|ClearandInvalidateTimerbyHandle _returnvalue_8))))

(fn ConstructionScript)

(fn CanInteractedInterfaceAnim
  (if (Variables|Default|GetIs%20sit?)
    (return false)
    (else
      (return true))))